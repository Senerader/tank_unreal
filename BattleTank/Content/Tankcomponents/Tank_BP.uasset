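; Player-drivable tank pawn Blueprint that wires its components to C++ aiming and movement components and routes player input to them.
; On BeginPlay it hands the turret and barrel to TankAiming and both tracks to TankMovement for initialization.
; Aim axes rotate an azimuth gimbal and spring arm to orbit the camera, while move axes send intents to TankMovement and the fire button calls TankAiming.Fire.
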(event `self.ReceiveBeginPlay`
  ;[1 1 1] Setting up the barrel, turret and movement component in C++
  (`TankAimingComponent.Initialize` (`self.TankAiming`) (`self.TankTurret`) (`self.TankBarrel`))
  (`TankMovementComponent.Initialize` (`self.TankMovement`) (`self.TankTrackL`) (`self.TankTrackR`)))

(event `InputAxis|AimElevation`
  (params (AxisValue :type "Float (single-precision)"))
  ;[1 1 1] Camera Elevation SpringArm
  (`SceneComponent.K2_AddLocalRotation` (`self.SpringArm`) (`KismetMathLibrary.MakeRotator` 0.0 AxisValue) false false))

(event `InputAxis|AimAzimuth`
  (params (AxisValue :type "Float (single-precision)"))
  ;[1 1 1] Camera yaw Azimuth Gimbal
  (`SceneComponent.K2_AddLocalRotation` (`self.azimuth gimbal`) (`KismetMathLibrary.MakeRotator` 0.0 0.0 AxisValue) false false))

(event `InputAxis|MoveForward`
  (params (AxisValue :type "Float (single-precision)"))
  ;[1 1 1] Input Tack Throttle
  (`TankMovementComponent.IntendMoveForward` (`self.TankMovement`) AxisValue))

(event `InputAxis|MoveRight`
  (params (AxisValue :type "Float (single-precision)"))
  ;[1 1 1] Input Tack Throttle
  (`TankMovementComponent.IntendTurnRight` (`self.TankMovement`) AxisValue))

(event `InputAction|FireButton`
  (params (Key :type "Key Structure"))
  ;[1 1 1] Firing method call
  (:`Pressed`
    (`TankAimingComponent.Fire` (`self.TankAiming`))))

(fn `UserConstructionScript`
  ;[1 1 1] Constructing mesh components due to bug in BP reason
)